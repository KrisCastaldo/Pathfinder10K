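; In-world terminal that shows a widget screen when the first-person character enters its box, either as a logic gate puzzle or a text terminal.
; Overlap swaps the screen material to glass and starts the character's mouse-follow timer; leaving reverts this and restores the first-person camera.
; In logic gate mode, an optional pressure plate gates trash spawning from linked chutes and its prompt.
; Victory replaces the widget with a door-unlocked display and green material.
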(event OnComponentBeginOverlap(Box)
  (params (OverlappedComponent :type Primitive%20Component%20Object%20Reference) (OtherActor :type Actor%20Object%20Reference) (OtherComp :type Primitive%20Component%20Object%20Reference) (OtherBodyIndex :type Integer) (bFromSweep :type Boolean) (SweepResult :type Hit%20Result%20Structure%20%28by%20ref%29))
  (bind _returnvalue (Game|GetPlayerCharacter OtherActor))
  (bind _chuteref (Variables|Default|GetChuteRef))
  (bind _pressureplate (Variables|Default|GetPressurePlate))
  (bind _presse (Variables|Default|GetPressE))
  (bind _item (Utilities|Array|Get(acopy) _chuteref))
  ;[1 1 1] BeingOverlap
  (Variables|/Game/FirstPersonBP/Blueprints/FirstPersonCharacter.FirstPersonCharacter_C|SetLogicGateTerm (.AsFirst%20Person%20Character (Utilities|Casting|CastToFirstPersonCharacter OtherActor)) self)
  (if (Variables|Default|GetLogicGate)
    (CallFunction|ShowLogic _returnvalue)
    (if (!= _pressureplate 0)
      (if (not (Variables|/Game/Interactables/WeightButton.WeightButton_C|GetStepped%20On _pressureplate))
        (Variables|Default|SetCanSpawn true :!label _label)
        (if (Variables|Default|GetShowTxt)
          (if (!= _item 0)
            (Rendering|SetVisibility _presse true false)
            (if (Variables|/Game/Interactables/TrashChute.TrashChute_C|GetCube? _item)
              (Rendering|Components|TextRender|SetText _presse (Variables|Default|GetCubeTxt))
              (else
                (Rendering|Components|TextRender|SetText _presse (Variables|Default|GetSphereTxt)))))))
      (else
        (goto _label)))
    (else
      (CallFunction|ShowLogic _returnvalue))))

(event OnComponentEndOverlap(Box)
  (params (OverlappedComponent :type Primitive%20Component%20Object%20Reference) (OtherActor :type Actor%20Object%20Reference) (OtherComp :type Primitive%20Component%20Object%20Reference) (OtherBodyIndex :type Integer))
  (bind _returnvalue (Game|GetPlayerCharacter OtherActor))
  ;[1 1 1] EndOverlap
  (Variables|/Game/FirstPersonBP/Blueprints/FirstPersonCharacter.FirstPersonCharacter_C|SetLogicGateTerm (.AsFirst%20Person%20Character (Utilities|Casting|CastToFirstPersonCharacter OtherActor)) 0)
  (if (Variables|Default|GetLogicGate)
    (CallFunction|HideLogic _returnvalue)
    (Variables|Default|SetCanSpawn false)
    (Rendering|SetVisibility (Variables|Default|GetPressE) false false)
    (else
      (CallFunction|HideLogic _returnvalue))))

(event Custom|TxtTerm
  ;[1 1 1] Set As Text
  (bind _returnvalue (UserInterface|CreateWidget (Variables|Default|GetTheLogicGate)))
  (bind _output_get (Variables|Default|SetRef _returnvalue))
  (UserInterface|SetWidget (Variables|Default|GetWidget) _returnvalue)
  (Widget|SetVisibility _output_get "Hidden"))

(event Custom|Show%20Logic
  (params (Object :type Object%20Object%20Reference))
  (bind _asfirst_person_character (Utilities|Casting|CastToFirstPersonCharacter Object))
  ;[1 1 1] Show Logic
  (Rendering|Material|SetMaterial (Variables|Default|GetCube) 0 "/Game/StarterContent/Materials/M_Glass.M_Glass")
  (Widget|SetVisibility (Variables|Default|GetRef) "Visible")
  (Utilities|Time|SetTimerbyFunctionName _asfirst_person_character "FollowMouse" 0.01 true)
  (Default|StartOpacity _asfirst_person_character self))

(event Custom|Victory
  ;[1 1 1] Display Door Unlocked screen and remove Logic Gate
  (Rendering|SetVisibility (Variables|Default|GetDoorUnlocked) true false)
  (Rendering|SetVisibility (Variables|Default|GetWidget) false false)
  (bind _output_get (Variables|Default|SetoriginalMat "/Game/Imported_Art/Terminal/Texture/Terminal_M_Green.Terminal_M_Green"))
  (Rendering|Material|SetMaterial (Variables|Default|GetCube) 0 _output_get))

(event Custom|Hide%20Logic
  (params (Object :type Object%20Object%20Reference))
  (bind _asfirst_person_character (Utilities|Casting|CastToFirstPersonCharacter Object))
  ;[1 1 1] Hide Logic
  (Variables|Default|SetCan%20Cursor false)
  (Rendering|Material|SetMaterial (Variables|Default|GetCube) 0 (Variables|Default|GetoriginalMat))
  (Widget|SetVisibility (Variables|Default|GetRef) "Hidden")
  (Utilities|Time|ClearTimerbyFunctionName _asfirst_person_character "FollowMouse")
  (Variables|/Game/FirstPersonBP/Blueprints/FirstPersonCharacter.FirstPersonCharacter_C|SetUnlockMouse _asfirst_person_character false)
  (Variables|/Script/UMG.WidgetInteractionComponent|SetbShowDebug (Variables|/Game/FirstPersonBP/Blueprints/FirstPersonCharacter.FirstPersonCharacter_C|GetWidgetInteraction _asfirst_person_character) false)
  (Utilities|Time|ClearTimerbyFunctionName _asfirst_person_character "WidgetOpacity")
  (Components|Activation|SetActive (Variables|/Game/FirstPersonBP/Blueprints/FirstPersonCharacter.FirstPersonCharacter_C|GetFirstPersonCamera _asfirst_person_character) true false)
  (Components|Activation|SetActive (Variables|/Game/FirstPersonBP/Blueprints/FirstPersonCharacter.FirstPersonCharacter_C|GetCameraToo _asfirst_person_character) false false))

(event Custom|LogicTerm
  ;[1 1 1] Set As Logic
  (bind _returnvalue (UserInterface|CreateWidget (Variables|Default|GetTheLogicGate)))
  (bind _output_get (Variables|Default|SetRef _returnvalue))
  (UserInterface|SetWidget (Variables|Default|GetWidget) _returnvalue)
  (Widget|SetVisibility _output_get "Hidden"))

(event Custom|CallChute
  (bind _chuteref (Variables|Default|GetChuteRef))
  ;[1 1 1] MakeTrash
  (if (Variables|Default|GetCanSpawn)
    (for _array_element _chuteref
      (Default|MakeTrash _array_element))
    (else
      (for _array_element_2 _chuteref
        (Default|Subtrash _array_element_2)))))

(event EventBeginPlay
  ;[1 1 1] Widget Or Text?
  (Variables|Default|SetoriginalMat (Rendering|Material|GetMaterial (Variables|Default|GetCube) 0))
  (Rendering|SetVisibility (Variables|Default|GetPressE) false false)
  (if (Variables|Default|GetLogicGate)
    (CallFunction|LogicTerm)
    (else
      (CallFunction|TxtTerm))))

(fn ConstructionScript)